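; BP_PlayerPawn is the player pawn, armed with a rifle that fires on left mouse press.
; On BeginPlay it spawns a BP_Rifle owned by itself, stores it as CurrentWeapon and snaps it to the mesh's WeaponSocket.
; When the SHealth component reports a health change, it briefly draws the delta as debug text at the pawn's location.
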(event OnHealthChanged(SHealth)
  (params (HealthComp :type S%20Health%20Component%20Object%20Reference) (Health :type Float%20%28single-precision%29) (HealthDelta :type Float%20%28single-precision%29) (DamageType :type Damage%20Type%20Object%20Reference) (InstigatedBy :type Controller%20Object%20Reference) (DamageCauser :type Actor%20Object%20Reference))
  (Rendering|Debug|DrawDebugString (Transformation|GetActorLocation) (Utilities|String|ToString(Float) HealthDelta) 0 "(R=1.000000,G=1.000000,B=1.000000,A=1.000000)" 1.0))

(event EventBeginPlay
  (bind _returnvalue (Game|SpawnActorfromClass "/Game/Blueprints/BP_Rifle.BP_Rifle_C" (Math|Transform|MakeTransform "0, 0, 0") "AlwaysSpawn" self 0))
  (Variables|Default|SetCurrentWeapon _returnvalue)
  (Transformation|AttachComponentToComponent _returnvalue (Variables|Character|GetMesh) "WeaponSocket" "SnapToTarget" "SnapToTarget" "SnapToTarget" true))

(event Collision|EventActorBeginOverlap
  (params (OtherActor :type Actor%20Object%20Reference)))

(event EventTick
  (params (DeltaSeconds :type Float%20%28single-precision%29)))

(event Input|MouseEvents|LeftMouseButton
  (params (Key :type Key%20Structure :default "None"))
  (:Pressed
    (Class|SWeapon|Fire (Variables|Default|GetCurrentWeapon))))

(fn ConstructionScript)